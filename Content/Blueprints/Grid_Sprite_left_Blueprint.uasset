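; Grid puzzle Blueprint with nine touchable boxes, each stepping its number upward to a cap of four to match a goal array.
; On touch, UpdateNumber destroys the overlapping actor and spawns the next number sprite at that box's hard-coded transform.
; DidIWin increments Score when the new value matches its goal, never decrements it, and prints a win message at eight, not nine.
; Hover events swap the cursor between hand and crosshairs.
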(event OnInputTouchBegin(Box9)
  (params (FingerIndex :type ETouchIndex%20Enum :default "Touch1") (TouchedComponent :type Primitive%20Component%20Object%20Reference))
  ;[1 1 1] Click Events
  (bind _new_box_int (CallFunction|UpdateNumber (Variables|GridInts|GetcurrentBox9) (Variables|Default|GetBox9) (|Box9Transform)))
  (bind _output_get (Variables|GridInts|SetcurrentBox9 _new_box_int))
  (CallFunction|DidIWin? _output_get (Utilities|Array|Get(acopy) (Variables|GridInts|GetintArrayGoal) 8) (Variables|Default|GetScore)))

(event OnBeginCursorOver(Box1)
  (params (TouchedComponent :type Primitive%20Component%20Object%20Reference))
  ;[1 1 1] Hover Effect
  (Variables|/Script/Engine.PlayerController|SetCurrentMouseCursor (Game|GetPlayerController 0) "Hand"))

(event OnEndCursorOver(Box1)
  (params (TouchedComponent :type Primitive%20Component%20Object%20Reference))
  ;[1 1 1] Hover Effect
  (Variables|/Script/Engine.PlayerController|SetCurrentMouseCursor (Game|GetPlayerController 0) "Crosshairs"))

(event OnBeginCursorOver(Box2)
  (params (TouchedComponent :type Primitive%20Component%20Object%20Reference))
  ;[1 1 1] Hover Effect
  (Variables|/Script/Engine.PlayerController|SetCurrentMouseCursor (Game|GetPlayerController 0) "Hand"))

(event OnEndCursorOver(Box2)
  (params (TouchedComponent :type Primitive%20Component%20Object%20Reference))
  ;[1 1 1] Hover Effect
  (Variables|/Script/Engine.PlayerController|SetCurrentMouseCursor (Game|GetPlayerController 0) "Crosshairs"))

(event OnBeginCursorOver(Box3)
  (params (TouchedComponent :type Primitive%20Component%20Object%20Reference))
  ;[1 1 1] Hover Effect
  (Variables|/Script/Engine.PlayerController|SetCurrentMouseCursor (Game|GetPlayerController 0) "Hand"))

(event OnEndCursorOver(Box3)
  (params (TouchedComponent :type Primitive%20Component%20Object%20Reference))
  ;[1 1 1] Hover Effect
  (Variables|/Script/Engine.PlayerController|SetCurrentMouseCursor (Game|GetPlayerController 0) "Crosshairs"))

(event OnBeginCursorOver(Box4)
  (params (TouchedComponent :type Primitive%20Component%20Object%20Reference))
  ;[1 1 1] Hover Effect
  (Variables|/Script/Engine.PlayerController|SetCurrentMouseCursor (Game|GetPlayerController 0) "Hand"))

(event OnInputTouchBegin(Box1)
  (params (FingerIndex :type ETouchIndex%20Enum :default "Touch1") (TouchedComponent :type Primitive%20Component%20Object%20Reference))
  ;[1 1 1] Click Events
  (bind _new_box_int (CallFunction|UpdateNumber (Variables|GridInts|GetcurrentBox1) (Variables|Default|GetBox1) (|Box1Tranform)))
  (bind _output_get (Variables|GridInts|SetcurrentBox1 _new_box_int))
  (CallFunction|DidIWin? _output_get (Utilities|Array|Get(acopy) (Variables|GridInts|GetintArrayGoal)) (Variables|Default|GetScore)))

(event OnEndCursorOver(Box4)
  (params (TouchedComponent :type Primitive%20Component%20Object%20Reference))
  ;[1 1 1] Hover Effect
  (Variables|/Script/Engine.PlayerController|SetCurrentMouseCursor (Game|GetPlayerController 0) "Crosshairs"))

(event OnBeginCursorOver(Box5)
  (params (TouchedComponent :type Primitive%20Component%20Object%20Reference))
  ;[1 1 1] Hover Effect
  (Variables|/Script/Engine.PlayerController|SetCurrentMouseCursor (Game|GetPlayerController 0) "Hand"))

(event OnEndCursorOver(Box5)
  (params (TouchedComponent :type Primitive%20Component%20Object%20Reference))
  ;[1 1 1] Hover Effect
  (Variables|/Script/Engine.PlayerController|SetCurrentMouseCursor (Game|GetPlayerController 0) "Crosshairs"))

(event OnBeginCursorOver(Box6)
  (params (TouchedComponent :type Primitive%20Component%20Object%20Reference))
  ;[1 1 1] Hover Effect
  (Variables|/Script/Engine.PlayerController|SetCurrentMouseCursor (Game|GetPlayerController 0) "Hand"))

(event OnEndCursorOver(Box6)
  (params (TouchedComponent :type Primitive%20Component%20Object%20Reference))
  ;[1 1 1] Hover Effect
  (Variables|/Script/Engine.PlayerController|SetCurrentMouseCursor (Game|GetPlayerController 0) "Crosshairs"))

(event OnBeginCursorOver(Box7)
  (params (TouchedComponent :type Primitive%20Component%20Object%20Reference))
  ;[1 1 1] Hover Effect
  (Variables|/Script/Engine.PlayerController|SetCurrentMouseCursor (Game|GetPlayerController 0) "Hand"))

(event OnEndCursorOver(Box7)
  (params (TouchedComponent :type Primitive%20Component%20Object%20Reference))
  ;[1 1 1] Hover Effect
  (Variables|/Script/Engine.PlayerController|SetCurrentMouseCursor (Game|GetPlayerController 0) "Crosshairs"))

(event OnBeginCursorOver(Box8)
  (params (TouchedComponent :type Primitive%20Component%20Object%20Reference))
  ;[1 1 1] Hover Effect
  (Variables|/Script/Engine.PlayerController|SetCurrentMouseCursor (Game|GetPlayerController 0) "Hand"))

(event OnEndCursorOver(Box8)
  (params (TouchedComponent :type Primitive%20Component%20Object%20Reference))
  ;[1 1 1] Hover Effect
  (Variables|/Script/Engine.PlayerController|SetCurrentMouseCursor (Game|GetPlayerController 0) "Crosshairs"))

(event OnInputTouchBegin(Box2)
  (params (FingerIndex :type ETouchIndex%20Enum :default "Touch1") (TouchedComponent :type Primitive%20Component%20Object%20Reference))
  ;[1 1 1] Click Events
  (bind _new_box_int (CallFunction|UpdateNumber (Variables|GridInts|GetcurrentBox2) (Variables|Default|GetBox2) (|Box2Transform)))
  (bind _output_get (Variables|GridInts|SetcurrentBox2 _new_box_int))
  (CallFunction|DidIWin? _output_get (Utilities|Array|Get(acopy) (Variables|GridInts|GetintArrayGoal) 1) (Variables|Default|GetScore)))

(event OnBeginCursorOver(Box9)
  (params (TouchedComponent :type Primitive%20Component%20Object%20Reference))
  ;[1 1 1] Hover Effect
  (Variables|/Script/Engine.PlayerController|SetCurrentMouseCursor (Game|GetPlayerController 0) "Hand"))

(event OnInputTouchBegin(Box3)
  (params (FingerIndex :type ETouchIndex%20Enum :default "Touch1") (TouchedComponent :type Primitive%20Component%20Object%20Reference))
  ;[1 1 1] Click Events
  (bind _new_box_int (CallFunction|UpdateNumber (Variables|GridInts|GetcurrentBox3) (Variables|Default|GetBox3) (|Box3Transform)))
  (bind _output_get (Variables|GridInts|SetcurrentBox3 _new_box_int))
  (CallFunction|DidIWin? _output_get (Utilities|Array|Get(acopy) (Variables|GridInts|GetintArrayGoal) 2) (Variables|Default|GetScore)))

(event OnEndCursorOver(Box9)
  (params (TouchedComponent :type Primitive%20Component%20Object%20Reference))
  ;[1 1 1] Hover Effect
  (Variables|/Script/Engine.PlayerController|SetCurrentMouseCursor (Game|GetPlayerController 0) "Crosshairs"))

(event OnInputTouchBegin(Box4)
  (params (FingerIndex :type ETouchIndex%20Enum :default "Touch1") (TouchedComponent :type Primitive%20Component%20Object%20Reference))
  ;[1 1 1] Click Events
  (bind _new_box_int (CallFunction|UpdateNumber (Variables|GridInts|GetcurrentBox4) (Variables|Default|GetBox4) (|Box4Transform)))
  (bind _output_get (Variables|GridInts|SetcurrentBox4 _new_box_int))
  (CallFunction|DidIWin? _output_get (Utilities|Array|Get(acopy) (Variables|GridInts|GetintArrayGoal) 3) (Variables|Default|GetScore)))

(event OnInputTouchBegin(Box5)
  (params (FingerIndex :type ETouchIndex%20Enum :default "Touch1") (TouchedComponent :type Primitive%20Component%20Object%20Reference))
  ;[1 1 1] Click Events
  (bind _new_box_int (CallFunction|UpdateNumber (Variables|GridInts|GetcurrentBox5) (Variables|Default|GetBox5) (|Box5Transform)))
  (bind _output_get (Variables|GridInts|SetcurrentBox5 _new_box_int))
  (CallFunction|DidIWin? _output_get (Utilities|Array|Get(acopy) (Variables|GridInts|GetintArrayGoal) 4) (Variables|Default|GetScore)))

(event OnInputTouchBegin(Box6)
  (params (FingerIndex :type ETouchIndex%20Enum :default "Touch1") (TouchedComponent :type Primitive%20Component%20Object%20Reference))
  ;[1 1 1] Click Events
  (bind _new_box_int (CallFunction|UpdateNumber (Variables|GridInts|GetcurrentBox6) (Variables|Default|GetBox6) (|Box6Transform)))
  (bind _output_get (Variables|GridInts|SetcurrentBox6 _new_box_int))
  (CallFunction|DidIWin? _output_get (Utilities|Array|Get(acopy) (Variables|GridInts|GetintArrayGoal) 5) (Variables|Default|GetScore)))

(event OnInputTouchBegin(Box7)
  (params (FingerIndex :type ETouchIndex%20Enum :default "Touch1") (TouchedComponent :type Primitive%20Component%20Object%20Reference))
  ;[1 1 1] Click Events
  (bind _new_box_int (CallFunction|UpdateNumber (Variables|GridInts|GetcurrentBox7) (Variables|Default|GetBox7) (|Box7Transform)))
  (bind _output_get (Variables|GridInts|SetcurrentBox7 _new_box_int))
  (CallFunction|DidIWin? _output_get (Utilities|Array|Get(acopy) (Variables|GridInts|GetintArrayGoal) 6) (Variables|Default|GetScore)))

(event OnInputTouchBegin(Box8)
  (params (FingerIndex :type ETouchIndex%20Enum :default "Touch1") (TouchedComponent :type Primitive%20Component%20Object%20Reference))
  ;[1 1 1] Click Events
  (bind _new_box_int (CallFunction|UpdateNumber (Variables|GridInts|GetcurrentBox8) (Variables|Default|GetBox8) (|Box8Transform)))
  (bind _output_get (Variables|GridInts|SetcurrentBox8 _new_box_int))
  (CallFunction|DidIWin? _output_get (Utilities|Array|Get(acopy) (Variables|GridInts|GetintArrayGoal) 7) (Variables|Default|GetScore)))

(fn ConstructionScript)

(fn UpdateNumber
  (params (Box%20int :type Integer) (Box%20Collision :type Box%20Component%20Object%20Reference) (Transform :type Transform))
  (if (< Box%20int 4)
    (bind _result (Math|Integer|IncrementInt Box%20int)
      (:%20%20
        (Actor|DestroyActor (Collision|GetOverlappingActors Box%20Collision 0 :!class /Script/Engine.PrimitiveComponent))
        (Game|SpawnActorfromClass (Utilities|Array|Get(acopy) (Variables|Default|GetnumberSprite) Box%20int) Transform "Undefined" 0 0)
        (return _result)))
    (else
      (return Box%20int))))

(fn DidIWin?
  (params (Current%20Box :type Integer) (Goal :type Integer) (Current%20Score :type Integer))
  (if (== Current%20Box Goal)
    (bind _result (Math|Integer|IncrementInt Current%20Score)
      (:%20%20
        (Variables|Default|SetScore _result)
        (if (== _result 8)
          (Development|PrintString "You Won!!!")
          (return true)
          (else
            (return false)))))
    (else
      (return false))))