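; Grid_Sprite_right is a Blueprint that places number-keyed child actors at given locations, apparently as part of a sprite grid.
; SpawnNumber switches on an integer from zero to four, and each branch adds its own Child Actor Component at the supplied location.
; The construction script is empty, and the file shows neither the child classes nor any caller of the function.
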(fn ConstructionScript)

(fn SpawnNumber
  (params (location :type Vector) (number :type Integer))
  (switch int number
    (:0
      (AddComponent|AddChildActorComponent false (Math|Conversions|ToTransform(Vector) location)))
    (:1
      (AddComponent|AddChildActorComponent false (Math|Conversions|ToTransform(Vector) location)))
    (:2
      (AddComponent|AddChildActorComponent false (Math|Conversions|ToTransform(Vector) location)))
    (:3
      (AddComponent|AddChildActorComponent false (Math|Conversions|ToTransform(Vector) location)))
    (:4
      (AddComponent|AddChildActorComponent false (Math|Conversions|ToTransform(Vector) location))))
  (return))