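; Grid sprite Blueprint, the "right" variant, that spawns a child actor to represent a number at a given location.
; Spawn Number switches on the number, handling zero through four, and each case adds its own Child Actor component at the supplied location.
; The construction script is empty, and other numbers have no case.
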(fn ConstructionScript)

(fn SpawnNumber
  (params (Location :type Vector) (number :type Integer))
  (switch int number
    (:0
      (AddComponent|AddChildActorComponent false (Math|Conversions|ToTransform(Vector) Location)))
    (:1
      (AddComponent|AddChildActorComponent false (Math|Conversions|ToTransform(Vector) Location)))
    (:2
      (AddComponent|AddChildActorComponent false (Math|Conversions|ToTransform(Vector) Location)))
    (:3
      (AddComponent|AddChildActorComponent false (Math|Conversions|ToTransform(Vector) Location)))
    (:4
      (AddComponent|AddChildActorComponent false (Math|Conversions|ToTransform(Vector) Location))))
  (return))